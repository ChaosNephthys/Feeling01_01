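; Diggable ground block that breaks when hit by the dig action of the referenced Action01.
; Each Tick, the active dig direction (default, up or down) selects which Action01 collision to test against DigActionCollision, draining one ObjectLife per overlapping frame.
; At zero life, a DoOnce-guarded event destroys only the visual ShapeCube component.
; Destructible-mesh damage, gravity, collision change and delayed actor destruction are present but never run.
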(event Custom|Destroy%20Object
  (Utilities|FlowControl|DoOnce false :!pinned true ; 一度のみ実行する
    (:Completed
      ;[1 1 1] Shape_Cube(見た目用)の消去
      (Components|DestroyComponent (Variables|Default|GetShape_Cube)))))

(event EventTick
  (params (DeltaSeconds :type Float%20%28single-precision%29))
  (bind _action01 (Variables|Default|GetAction01))
  (bind _action01_2 (Variables|Default|GetAction01))
  (bind _digactioncollision (Variables|Default|GetDigActionCollision))
  ;[1 1 1] 接触イベントをプレイヤー&掘るアクション中に限定
  (if (Variables|/Game/2DSideScrollerBP/Blueprints/2DSideScrollerCharacter.2DSideScrollerCharacter_C|GetAction01 _action01)
    (if (Class|PrimitiveComponent|IsOverlappingComponent _digactioncollision (Variables|/Game/2DSideScrollerBP/Blueprints/2DSideScrollerCharacter.2DSideScrollerCharacter_C|GetDigActionCollision _action01_2))
      ;[1 1 1] オブジェクトのライフを減らす
      (Variables|Default|SetObjectLife (- (Variables|Default|GetObjectLife) 1) :!label _label)
      (if (<= (Variables|Default|GetObjectLife) 0)
        (CallFunction|DestroyObject)))
    (elif (Variables|/Game/2DSideScrollerBP/Blueprints/2DSideScrollerCharacter.2DSideScrollerCharacter_C|GetAction01UP _action01)
      (if (Class|PrimitiveComponent|IsOverlappingComponent _digactioncollision (Variables|/Game/2DSideScrollerBP/Blueprints/2DSideScrollerCharacter.2DSideScrollerCharacter_C|GetDigActionCollisionUP _action01_2))
        (goto _label))
      (elif (Variables|/Game/2DSideScrollerBP/Blueprints/2DSideScrollerCharacter.2DSideScrollerCharacter_C|GetAction01DOWN _action01)
        (if (Class|PrimitiveComponent|IsOverlappingComponent _digactioncollision (Variables|/Game/2DSideScrollerBP/Blueprints/2DSideScrollerCharacter.2DSideScrollerCharacter_C|GetDigActionCollisionDOWN _action01_2))
          (goto _label))))))

(fn ConstructionScript)