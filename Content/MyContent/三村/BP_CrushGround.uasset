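; BP_CrushGround is a breakable ground block that the player destroys by digging.
; Each Tick, overlap with the player's dig collision during Action01 lowers ObjectLife, so durability is frame-rate dependent.
; At zero, a DoOnce removes the visible cube, damages the destructible mesh ShapeCubeDM and enables its gravity.
; Short delays then switch the debris to physics-only collision and destroy the actor.
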(event Custom|Destroy%20Object
  (bind _shape_cube_dm (Variables|Default|GetShape_Cube_DM))
  (bind _returnvalue (Transformation|GetWorldLocation _shape_cube_dm))
  (Utilities|FlowControl|DoOnce false :!pinned true ; 一度のみ実行する
    (:Completed
      ;[1 1 1] ShapeCube_DMにダメージ
      (Class|DestructibleComponent|ApplyDamage _shape_cube_dm 1e+01 _returnvalue _returnvalue 5e+02)
      ;[1 1 1] Shape_Cube(見た目用)の消去
      (Components|DestroyComponent (Variables|Default|GetShape_Cube))
      ;[1 1 1] 重力付与
      (Physics|SetEnableGravity (Variables|Default|GetShape_Cube_DM) true)
      ;[1 1 1] 0.1秒後にコリジョンをPhysics Onlyにする
      (Utilities|FlowControl|Delay 0.1)
      (Collision|SetCollisionEnabled (Variables|Default|GetShape_Cube_DM) "PhysicsOnly")
      ;[1 1 1] ２秒後このアクタを消去
      (Utilities|FlowControl|Delay 1.0)
      (Actor|DestroyActor))))

(event EventTick
  (params (DeltaSeconds :type Float%20%28single-precision%29))
  ;[1 1 1] 接触イベントをプレイヤー&掘るアクション中に限定
  (if (Class|PrimitiveComponent|IsOverlappingComponent (Variables|Default|GetDigActionCollision) (Variables|/Game/2DSideScrollerBP/Blueprints/2DSideScrollerCharacter.2DSideScrollerCharacter_C|GetDigActionCollision (Variables|Default|GetAction01)))
    (if (Variables|/Game/2DSideScrollerBP/Blueprints/2DSideScrollerCharacter.2DSideScrollerCharacter_C|GetAction01 (Variables|Default|GetAction01))
      ;[1 1 1] オブジェクトのライフを減らす
      (Variables|Default|SetObjectLife (- (Variables|Default|GetObjectLife) 1))
      (if (<= (Variables|Default|GetObjectLife) 0)
        (CallFunction|DestroyObject)))))

(fn ConstructionScript)