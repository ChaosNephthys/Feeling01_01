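; Side-view camera actor that becomes the player's view target on BeginPlay and follows the player pawn each tick.
; It tracks the pawn at a fixed Y offset while the pawn is between the LeftEnd and RightEnd actors, otherwise following only its height.
; HitStopEvent triggers a brief frame-counted shake that cycles diagonal X/Z offsets after the follow update, without pausing gameplay.
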(event Custom|HitStopEvent
  ;[1 1 1] HitStop&揺れ関連
  (Variables|Default|SetHitStopFlag true))

(event Custom|CameraFlow
  (bind _returnvalue (Game|Player|GetPlayerPawn 0))
  (bind _returnvalue_2 (Game|Player|GetPlayerPawn 0))
  (bind _self self)
  (bind _returnvalue_3 (Transformation|GetActorLocation _returnvalue))
  (bind _returnvalue_4 (Transformation|GetActorLocation _returnvalue_2))
  (bind _returnvalue_5 (Transformation|GetActorLocation _self))
  (bind _x (Math|Vector|BreakVector _returnvalue_4))
  (bind (_x_2 _y) (Math|Vector|BreakVector _returnvalue_5))
  ;[1 1 1] プレイヤーを追う処理
  (if (< (.X (Math|Vector|BreakVector (Transformation|GetActorLocation (Variables|Default|GetLeftEnd)))) _x)
    (if (> (.X (Math|Vector|BreakVector (Transformation|GetActorLocation (Variables|Default|GetRightEnd)))) _x)
      (Transformation|SetActorLocation (+ _returnvalue_3 "0,700.000000,0.000000") true false)
      (else
        (Transformation|SetActorLocation (Math|Vector|MakeVector _x_2 _y (.Z (Math|Vector|BreakVector _returnvalue_3))) true false :!label _label)))
    (else
      (goto _label))))

(event Custom|HitStopFlow
  (bind _self self)
  (bind _shakevalue (Variables|Default|GetShakeValue))
  (bind _returnvalue (Transformation|GetActorLocation _self))
  (bind (_x _y _z) (Math|Vector|BreakVector _returnvalue))
  (bind _returnvalue_2 (- _z _shakevalue))
  (bind _returnvalue_3 (- _x _shakevalue))
  (bind _returnvalue_4 (+ _x _shakevalue))
  (bind _returnvalue_5 (+ _z _shakevalue))
  ;[1 1 1] HitStop&揺れ関連
  (if (Variables|Default|GetHitStopFlag)
    (Variables|Default|SetHitStopCount (+ (Variables|Default|GetHitStopCount) 1))
    (if (> (Variables|Default|GetHitStopCount) 20)
      (Variables|Default|SetHitStopCount 0)
      (Variables|Default|SetHitStopFlag false)
      (else
        (switch int (/ (Math|Integer|%(Integer) (Variables|Default|GetHitStopCount) 8) 2)
          (:0
            (Transformation|SetActorLocation (Math|Vector|MakeVector _returnvalue_4 _y _returnvalue_5) true false))
          (:1
            (Transformation|SetActorLocation (Math|Vector|MakeVector _returnvalue_4 _y _returnvalue_2) true false))
          (:2
            (Transformation|SetActorLocation (Math|Vector|MakeVector _returnvalue_3 _y _returnvalue_5) true false))
          (:3
            (Transformation|SetActorLocation (Math|Vector|MakeVector _returnvalue_3 _y _returnvalue_2) true false)))))))

(event EventBeginPlay
  (Game|Player|SetViewTargetwithBlend (Game|GetPlayerController 0) self 0.0 "VTBlend_Linear" 0.0 false))

(event EventTick
  (params (DeltaSeconds :type Float%20%28single-precision%29))
  (CallFunction|CameraFlow)
  (CallFunction|HitStopFlow))

(fn ConstructionScript)