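; BP_CrushCore is a diggable core object that loses life while hit by the player's dig action, then shatters.
; Tick checks overlap with the player's dig collision for the active action (normal, up or down), decrementing life every qualifying frame.
; Non-lethal hits alternate two destructible meshes by life parity, resetting and fracturing each.
; At zero life it fractures, drops debris, removes components after short delays and triggers hit stop on BP_CharacterCamera.
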(event Custom|Destroy%20Object
  (bind _shape_cube_dm_core (Variables|Default|GetShape_Cube_DM_Core))
  (bind _returnvalue (Transformation|GetWorldLocation _shape_cube_dm_core))
  (Utilities|FlowControl|DoOnce false :!pinned true ; 一度のみ実行する
    (:Completed
      ;[1 1 1] ShapeCube_DMにダメージ
      (Class|DestructibleComponent|ApplyDamage _shape_cube_dm_core 5e+02 _returnvalue _returnvalue 5e+02)
      ;[1 1 1] Shape_Cube(見た目用)の消去
      (Components|DestroyComponent (Variables|Default|GetShape_Cube_DM_App))
      (Components|DestroyComponent (Variables|Default|GetShape_Cube_DM_Core2))
      ;[1 1 1] 重力付与
      (Physics|SetEnableGravity (Variables|Default|GetShape_Cube_DM_Core) true)
      ;[1 1 1] 0.1秒後にコリジョンをPhysics Onlyにする
      (Utilities|FlowControl|Delay 0.1)
      (Collision|SetCollisionEnabled (Variables|Default|GetShape_Cube_DM_Core) "PhysicsOnly")
      ;[1 1 1] ２秒後このコアを消去
      (Utilities|FlowControl|Delay 1.0)
      (Components|DestroyComponent (Variables|Default|GetShape_Cube_DM_Core)))))

(event Custom|Damage%20Effect
  (bind _shape_cube_dm_core (Variables|Default|GetShape_Cube_DM_Core))
  (bind _shape_cube_dm_core2 (Variables|Default|GetShape_Cube_DM_Core2))
  (bind _returnvalue (Transformation|GetWorldLocation _shape_cube_dm_core2))
  (bind _returnvalue_2 (Transformation|GetWorldLocation _shape_cube_dm_core))
  ;[1 1 1] 攻撃ごとに発生するエフェクト
  (if (== (Math|Integer|%(Integer) (Variables|Default|GetObjectLife) 2) 1)
    (Class|DestructibleComponent|SetDestructibleMesh _shape_cube_dm_core "/Game/MyContent/三村/Materials/素材/Shape_Cube_DM.Shape_Cube_DM")
    (Class|DestructibleComponent|ApplyDamage _shape_cube_dm_core 5e+02 _returnvalue_2 _returnvalue_2 3e+03)
    (else
      (Class|DestructibleComponent|SetDestructibleMesh _shape_cube_dm_core2 "/Game/MyContent/三村/Materials/素材/Shape_Cube_DM.Shape_Cube_DM")
      (Class|DestructibleComponent|ApplyDamage _shape_cube_dm_core2 5e+02 _returnvalue _returnvalue 3e+03))))

(event EventTick
  (params (DeltaSeconds :type Float%20%28single-precision%29))
  (bind _returnvalue (Game|Player|GetPlayerPawn 0))
  (bind _digactioncollision (Variables|Default|GetDigActionCollision))
  (bind _as2dside_scroller_character (Utilities|Casting|CastTo2DSideScrollerCharacter _returnvalue))
  ;[1 1 1] 接触イベントをプレイヤー&掘るアクション中に限定
  (if (Variables|/Game/2DSideScrollerBP/Blueprints/2DSideScrollerCharacter.2DSideScrollerCharacter_C|GetAction01 _as2dside_scroller_character)
    (if (Class|PrimitiveComponent|IsOverlappingComponent _digactioncollision (Variables|/Game/2DSideScrollerBP/Blueprints/2DSideScrollerCharacter.2DSideScrollerCharacter_C|GetDigActionCollision _as2dside_scroller_character))
      ;[1 1 1] オブジェクトのライフを減らす
      (Variables|Default|SetObjectLife (- (Variables|Default|GetObjectLife) 1) :!label _label)
      (if (== (Variables|Default|GetObjectLife) 0)
        (CallFunction|DestroyObject)
        (bind _outactors (Actor|GetAllActorsOfClass "/Game/MyContent/三村/BP/BP_CharacterCamera.BP_CharacterCamera_C"))
        (Default|HitStopEvent (Utilities|Array|Get(acopy) _outactors))
        (elif (> (Variables|Default|GetObjectLife) 0)
          (CallFunction|DamageEffect))))
    (elif (Variables|/Game/2DSideScrollerBP/Blueprints/2DSideScrollerCharacter.2DSideScrollerCharacter_C|GetAction01UP _as2dside_scroller_character)
      (if (Class|PrimitiveComponent|IsOverlappingComponent _digactioncollision (Variables|/Game/2DSideScrollerBP/Blueprints/2DSideScrollerCharacter.2DSideScrollerCharacter_C|GetDigActionCollisionUP _as2dside_scroller_character))
        (goto _label))
      (elif (Variables|/Game/2DSideScrollerBP/Blueprints/2DSideScrollerCharacter.2DSideScrollerCharacter_C|GetAction01DOWN _as2dside_scroller_character)
        (if (Class|PrimitiveComponent|IsOverlappingComponent _digactioncollision (Variables|/Game/2DSideScrollerBP/Blueprints/2DSideScrollerCharacter.2DSideScrollerCharacter_C|GetDigActionCollisionDOWN _as2dside_scroller_character))
          (goto _label))))))

(fn ConstructionScript)