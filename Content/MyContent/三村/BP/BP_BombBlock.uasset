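; BP_BombBlock is a bomb block that explodes when the player's dig action hits it.
; Each Tick checks the active dig state on Action01 (default, up or down) and tests whether the block's DigActionCollision overlaps the matching collision.
; On overlap, BombObject applies heavy damage and impulse to ShapeCubeDMCore, attaches an enlarged explosion emitter, then destroys the actor after a short delay.
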(event Custom|Bomb%20Object
  (bind _shape_cube_dm_core (Variables|Default|GetShape_Cube_DM_Core))
  (bind _returnvalue (Transformation|GetWorldLocation _shape_cube_dm_core))
  (Class|DestructibleComponent|ApplyDamage _shape_cube_dm_core 5e+02 _returnvalue _returnvalue 3e+04)
  (Effects|SpawnEmitterAttached "/Game/StarterContent/Particles/P_Explosion.P_Explosion" (Variables|Default|GetShape_Cube_DM_Core) "None" "0, 0, 0" "0, 0, 0" "5.000000,5.000000,5.000000")
  (Utilities|FlowControl|Delay 0.1)
  (Actor|DestroyActor))

(event EventTick
  (params (DeltaSeconds :type Float%20%28single-precision%29))
  (bind _digactioncollision (Variables|Default|GetDigActionCollision))
  (bind _action01 (Variables|Default|GetAction01))
  (bind _action01_2 (Variables|Default|GetAction01))
  ;[1 1 1] 接触イベントをプレイヤー&掘るアクション中に限定
  (if (Variables|/Game/2DSideScrollerBP/Blueprints/2DSideScrollerCharacter.2DSideScrollerCharacter_C|GetAction01 _action01)
    (if (Class|PrimitiveComponent|IsOverlappingComponent _digactioncollision (Variables|/Game/2DSideScrollerBP/Blueprints/2DSideScrollerCharacter.2DSideScrollerCharacter_C|GetDigActionCollision _action01_2))
      (CallFunction|BombObject :!label _label))
    (elif (Variables|/Game/2DSideScrollerBP/Blueprints/2DSideScrollerCharacter.2DSideScrollerCharacter_C|GetAction01UP _action01)
      (if (Class|PrimitiveComponent|IsOverlappingComponent _digactioncollision (Variables|/Game/2DSideScrollerBP/Blueprints/2DSideScrollerCharacter.2DSideScrollerCharacter_C|GetDigActionCollisionUP _action01_2))
        (goto _label))
      (elif (Variables|/Game/2DSideScrollerBP/Blueprints/2DSideScrollerCharacter.2DSideScrollerCharacter_C|GetAction01DOWN _action01)
        (if (Class|PrimitiveComponent|IsOverlappingComponent _digactioncollision (Variables|/Game/2DSideScrollerBP/Blueprints/2DSideScrollerCharacter.2DSideScrollerCharacter_C|GetDigActionCollisionDOWN _action01_2))
          (goto _label))))))

(fn ConstructionScript)